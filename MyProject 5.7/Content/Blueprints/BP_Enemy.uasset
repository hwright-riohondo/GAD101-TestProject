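; Enemy character that patrols between random tagged actors, pausing at each, and reacts to AI Perception.
; It speeds up to chase a perceived player and plays an attack montage on arrival, or investigates the location of "ball" stimuli.
; Forgetting a target restores walk speed and patrol.
; DetectHit sphere-traces at the right hand to hit the player; the enemy's OnHit plays a death montage and OnDead destroys it.
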(event OnTargetPerceptionUpdated(AIPerception)
  (params (Actor :type Actor%20Object%20Reference) (Stimulus :type AI%20Stimulus%20Structure))
  (bind (_age _expirationage _strength _stimuluslocation _receiverlocation _tag) (Utilities|Struct|BreakAIStimulus Stimulus))
  (if (not (== _tag "ball"))
    (bind _asphase_player_character (Utilities|Casting|CastToPhasePlayerCharacter Actor))
    (Variables|/Script/Engine.CharacterMovementComponent|SetMaxWalkSpeed (Variables|Character|GetCharacterMovement) 5e+02)
    (AI|AIMoveTo self "0, 0, 0" _asphase_player_character 5.0 false
      (:OnSuccess
        (Animation|PlayAnimMontage "/Game/Characters/Mannequins/Anims/Unarmed/Attack/MM_Attack_01_Montage.MM_Attack_01_Montage" 1.0 "None")))
    (else
      (AI|AIMoveTo self _stimuluslocation 0 5.0 false))))

(event OnTargetPerceptionForgotten(AIPerception)
  (params (Actor :type Actor%20Object%20Reference))
  (Variables|/Script/Engine.CharacterMovementComponent|SetMaxWalkSpeed (Variables|Character|GetCharacterMovement) 3e+02)
  (CallFunction|EventPatroltoNewPoint))

(event Custom|Event%20PatrolToNewPoint
  (AI|AIMoveTo self "0, 0, 0" (.OutItem (Utilities|Array|Random (Variables|Default|GetPatrolPoints))) 5.0 false
    (:OnSuccess
      (Utilities|FlowControl|Delay 3.0)
      (CallFunction|EventPatroltoNewPoint))))

(event Custom|OnHit
  (Animation|PlayAnimMontage "/Game/Characters/Mannequins/Anims/Phase/Animations/Death_Montage.Death_Montage" 1.0 "None"))

(event Custom|OnDead
  (Actor|DestroyActor))

(event EventBeginPlay
  (bind _outactors (Actor|GetAllActorswithTag (Variables|Default|GetTag)))
  (Variables|Default|SetPatrolPoints _outactors)
  (CallFunction|EventPatroltoNewPoint))

(event Collision|EventActorBeginOverlap
  (params (OtherActor :type Actor%20Object%20Reference)))

(event EventTick
  (params (DeltaSeconds :type Float%20%28single-precision%29)))

(fn ConstructionScript)

(fn DetectHit
  (bind _mesh (Variables|Character|GetMesh))
  (bind _returnvalue (Transformation|GetSocketLocation _mesh "hand_r"))
  (bind _outhit (Collision|SphereTraceForObjects _returnvalue _returnvalue 5e+01 (Utilities|Array|MakeArray "ObjectTypeQuery3") false 0 "ForDuration"))
  (bind _asphase_player_character (Utilities|Casting|CastToPhasePlayerCharacter (.HitActor (Collision|BreakHitResult _outhit))))
  (Default|OnHit _asphase_player_character))