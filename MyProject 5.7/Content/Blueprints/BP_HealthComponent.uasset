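; BP_HealthComponent is a health component that tracks hit points and processes incoming damage.
; ReceiveDamage subtracts the amount from current HP, clamped between zero and max HP, then updates the health percentage and the died flag.
; It then fires OnHealthChanged on every call, with no separate death notification.
; The event graph holds only disabled BeginPlay and Tick stubs, so all logic lives in that function.
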(fn `ReceiveDamage`
  (params (Amount :type "Float (double-precision)"))
  (bind _output_get (set `self.CurrentHP` (`KismetMathLibrary.FClamp` (- (`self.CurrentHP`) Amount) 0.0 (`self.MaxHP`))))
  (set `self.HealthPercentage` (/ _output_get (`self.MaxHP`)))
  (set `self.Died` (<= (`self.CurrentHP`) 0.0))
  (`self.OnHealthChanged`))